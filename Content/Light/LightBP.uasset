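; LightBP is a light fixture with a bulb mesh and a spotlight that flickers continuously from BeginPlay.
; The Flicker event chains randomized delays between two off/on blinks, then calls itself to loop indefinitely.
; TurnOff and TurnOn swap the bulb material between black and its lit material while toggling spotlight visibility to match.
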(event `Flicker`
  (`KismetSystemLibrary.Delay` (`KismetMathLibrary.RandomFloatInRange` 0.9 1.8) :!label _label)
  (`self.Turn Off`)
  (`KismetSystemLibrary.Delay` (`KismetMathLibrary.RandomFloatInRange` 0.1 0.8))
  (`self.Turn On`)
  (`KismetSystemLibrary.Delay` (`KismetMathLibrary.RandomFloatInRange` 0.1 0.5))
  (`self.Turn Off`)
  (`KismetSystemLibrary.Delay` (`KismetMathLibrary.RandomFloatInRange` 0.4 0.8))
  (`self.Turn On`)
  (`self.Flicker`))

(event `self.ReceiveBeginPlay`
  (goto _label))

(event `Turn Off`
  (`PrimitiveComponent.SetMaterial` (`self.LightBulb`) 0 "/Game/Materials/Black.Black")
  (`SceneComponent.SetVisibility` (`self.SpotLight`) false false))

(event `Turn On`
  (`PrimitiveComponent.SetMaterial` (`self.LightBulb`) 0 "/Game/Light/AM152_069_06.AM152_069_06")
  (`SceneComponent.SetVisibility` (`self.SpotLight`) true false))

(fn `UserConstructionScript`)